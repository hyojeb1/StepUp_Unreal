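; Gameplay ability for the Q attack, which damages the first target hit in front of the avatar.
; It commits cost, then sphere-traces on the Camera channel along the pawn's forward vector out to Range, with debug drawing.
; A hit applies GE_AttackQ_Damage through hit-result target data.
; The AttackQ gameplay cue fires at the trace's hit location even on a miss, then cooldown commits and the ability ends.
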(event Ability|EventActivateAbility
  (bind (_startlocation _endlocation) (CallFunction|GetActorStartandEnd))
  (Ability|CommitAbilityCost false)
  (bind (_outhit _returnvalue) (Collision|SphereTraceByChannel _startlocation _endlocation 5e+01 "TraceTypeQuery2" false (Utilities|Array|MakeArray (Ability|GetAvatarActorfromActorInfo)) "ForDuration" true "(R=1.000000,G=0.000000,B=0.000000,A=1.000000)" "(R=0.000000,G=1.000000,B=0.000000,A=1.000000)" 2.0))
  (if _returnvalue
    (GameplayEffects|ApplyGameplayEffectToTarget (Ability|TargetData|AbilityTargetDatafromHitResult _outhit) "/Game/GameAbilitySystem/Effects/GE_AttackQ_Damage.GE_AttackQ_Damage_C" 1 1))
  (Class|GameplayAbility|ExecuteGameplayCuewithParams "(TagName=\"GameplayCue.AttackQ.Active\")" (Ability|GameplayCue|MakeGameplayCueParameters :Location (.Location (Collision|BreakHitResult _outhit))))
  (Ability|CommitAbilityCooldown false)
  (Ability|EndAbility))

(event Ability|EventOnEndAbility
  (params (bWasCancelled :type Boolean)))

(fn GetActorStartandEnd
  (bind _aspawn (Utilities|Casting|CastToPawn (Ability|GetAvatarActorfromActorInfo))
    (:then
      (return (Transformation|GetActorLocation _aspawn) (+ (Transformation|GetActorLocation _aspawn) (* (Transformation|GetActorForwardVector _aspawn) (LocalVariables|GetRange)))))
    (:CastFailed
      (Development|PrintString "GA_Attak is Fucked!")
      (return "0, 0, 0" "0, 0, 0"))))