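; Gameplay ability for an attack that sphere-traces forward from the avatar pawn's location out to Range.
; Activation commits the cost, then traces on the Visibility channel, ignoring the avatar and drawing debug shapes.
; A hit adds a gameplay cue set to be removed on ability end, while only a miss commits the cooldown.
; Both paths end the ability immediately, and no damage is applied here.
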(event Ability|EventActivateAbility
  (bind (_startlocation _endlocation) (CallFunction|GetActorStartandEnd))
  (Ability|CommitAbilityCost false)
  (bind _returnvalue (Collision|SphereTraceByChannel _startlocation _endlocation 5e+01 "TraceTypeQuery1" false (Utilities|Array|MakeArray (Ability|GetAvatarActorfromActorInfo)) "ForDuration"))
  (if _returnvalue
    (GameplayCue|AddGameplayCue)
    (else
      (Ability|CommitAbilityCooldown false)))
  (Ability|EndAbility))

(event Ability|EventOnEndAbility
  (params (bWasCancelled :type Boolean)))

(fn GetActorStartandEnd
  (bind _aspawn (Utilities|Casting|CastToPawn (Ability|GetAvatarActorfromActorInfo))
    (:then
      (return (Transformation|GetActorLocation _aspawn) (+ (Transformation|GetActorLocation _aspawn) (* (Transformation|GetActorForwardVector _aspawn) (LocalVariables|GetRange)))))
    (:CastFailed
      (Development|PrintString "GA_Attak is Fucked!")
      (return "0, 0, 0" "0, 0, 0"))))